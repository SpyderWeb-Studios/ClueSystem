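; Clue actor Blueprint that represents an interactable clue, driven by a soft-referenced clue primary data asset.
; When LoadAndSetMesh is set, the construction script blocking-loads the asset, applies its mesh, then requests its unload.
; LoadClueAssetData loads the asset asynchronously and passes it to CallOnDataAssetLoaded.
; AttemptInteraction ignores the interactor and returns the result of AttemptInteractionWithClue.
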(event EventBeginPlay)

(event Collision|EventActorBeginOverlap
  (params (OtherActor :type Actor%20Object%20Reference)))

(event EventTick
  (params (DeltaSeconds :type Float%20%28single-precision%29)))

(event EventLoadClueAssetData
  (bind _object (Utilities|AsyncLoadAsset (Variables|Default|GetClueDataAsset))
    (:Completed
      (bind _asprimary_data_asset_clue (Utilities|Casting|CastToPrimaryDataAsset_Clue _object))
      (Default|CallOnDataAssetLoaded _asprimary_data_asset_clue))))

(fn ConstructionScript
  (if (Variables|Default|GetLoad%20And%20Set%20Mesh)
    (bind _returnvalue (Utilities|LoadAssetBlocking (Variables|Default|GetClueDataAsset)))
    (bind _asprimary_data_asset_clue (Utilities|Casting|CastToPrimaryDataAsset_Clue _returnvalue))
    (Components|StaticMesh|SetStaticMesh (Variables|Default|GetStaticMesh) (Variables|/Script/ClueSystem.PrimaryDataAsset_Clue|GetClueMesh _asprimary_data_asset_clue))
    (Class|KismetSystemLibrary|UnloadPrimaryAsset (AssetManager|GetPrimaryAssetIdfromObject _asprimary_data_asset_clue))))

(fn AttemptInteraction
  (params (Interactor :type Interact%20Component%20Object%20Reference))
  (bind _returnvalue (Class|ClueBase|AttemptInteractionwithClue))
  (return _returnvalue))